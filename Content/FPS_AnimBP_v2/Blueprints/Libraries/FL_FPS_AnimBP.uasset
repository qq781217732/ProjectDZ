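; Blueprint function library of shared helpers for the FPS AnimBP project.
; Input device and HUD helpers message the first player controller and classify keys as keyboard/mouse or gamepad.
; Other helpers validate weapon attachments against slot, asset and gun restrictions, and synchronously load and cast soft animation, sound and mesh references.
; Surface responses come from matching hit physical materials to DataTable rows, with optional debug output through a color-coded message printer.
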(fn `Display Error Message`
  (params (Message :type String) (`Self Object` :type "Object Object Reference") (`Function Name` :type String) (Urgency :type "/Game/FPS_AnimBP_v2/Data/Enums/E_ErrorMessageUrgency Enum" :default "NewEnumerator0") (bPrintToScreen :type Boolean) (bPrintToLog :type Boolean) (Duration :type "Float (double-precision)"))
  (locals (local_String :type String) (local_TextColor :type "LinearColor Structure"))
  ;[0 0 0] Prints a unified error message with the class and function named specified if desired
  (set `local.local_String` (`KismetStringLibrary.Concat_StrStr` Message " \n" (`KismetSystemLibrary.GetClassDisplayName` (`GameplayStatics.GetObjectClass` `Self Object`)) " > " `Function Name`))
  (set `local.local_TextColor` (select `/Game/FPS_AnimBP_v2/Data/Enums/E_ErrorMessageUrgency` (`local.Urgency`) :`NewEnumerator0` (struct :`R` 0.63688 :`G` 1.0 :`A` 1.0) :`NewEnumerator1` (struct :`R` 1.0 :`G` 0.442751 :`A` 1.0) :`NewEnumerator2` (struct :`R` 1.0 :`A` 1.0) :!type "LinearColor Structure"))
  (`KismetSystemLibrary.PrintString` null (`local.local_String`) (`local.bPrintToScreen`) (`local.bPrintToLog`) (`local.local_TextColor`) (`local.Duration`)))

(fn `Get Physical Material Response By Surface Type`
  (params (`Data Table` :type "DataTable Object Reference") (Hit :type "HitResult Structure (by ref)") (`Owning Object` :type "Object Object Reference") (`Display Physical Material Details` :type Boolean))
  (returns (PhysMatRespons :type "/Game/FPS_AnimBP_v2/Data/Structs/ST_PhysMatResponse Structure"))
  (locals (local_PhysMatResponse :type "/Game/FPS_AnimBP_v2/Data/Structs/ST_PhysMatResponse Structure"))
  (bind _hit (`local.Hit`))
  ;[0 0 0] Select the Physical Material Response struct based on the Physical Material assigned to the hit surface
  (bind _outrownames (`DataTableFunctionLibrary.GetDataTableRowNames` `Data Table`))
  (for _array_element _outrownames
    (bind _returnvalue (`|GetDataTableRow` (`local.Data Table`) _array_element)
      (:`then`
        (if (== (`.PhysicalMaterial_7_8D34A19D471F3560FA0A8394494FBD5B` (break `/Game/FPS_AnimBP_v2/Data/Structs/ST_PhysMatResponse` _returnvalue)) (`.PhysMat` (`GameplayStatics.BreakHitResult` (`local.Hit`))))
          (set `local.local_PhysMatResponse` _returnvalue)
          (break)))))
  (if (`local.Display Physical Material Details`)
    (`self.Display Error Message` (`KismetStringLibrary.Concat_StrStr` "Surface Type " (`|GetEnumeratorNameAsString` (`GameplayStatics.GetSurfaceType` _hit)) " \nMaterial: " (`KismetSystemLibrary.GetDisplayName` (`.PhysMat` (`GameplayStatics.BreakHitResult` _hit)))) (`local.Owning Object`) "FL_FPS_AnimBP > GetImpactDecalBySurfaceType" "NewEnumerator0" true false 3.0))
  (return (`local.local_PhysMatResponse`)))

(fn `GetCurrentInputDevice`
  (returns (InputDevice :type "/Game/FPS_AnimBP_v2/Data/Enums/E_InputDevice Enum"))
  (bind _inputdevice (message `/Game/FPS_AnimBP_v2/Blueprints/Interfaces/BP_ControllerInterface.GetInputDevice` (`GameplayStatics.GetPlayerController` null)))
  (return _inputdevice))

(fn `GetInputDeviceByKey`
  (params (Key :type "Key Structure (by ref)"))
  (returns (`Input Device` :type "/Game/FPS_AnimBP_v2/Data/Enums/E_InputDevice Enum"))
  ;[0 0 0] Get the current input device based on the last input received
  (if (or (`KismetInputLibrary.Key_IsKeyboardKey` Key) (`KismetInputLibrary.Key_IsMouseButton` Key))
    (return "NewEnumerator0")
    (elif (`KismetInputLibrary.Key_IsGamepadKey` Key)
      (return "NewEnumerator1"))))

(fn `GetPlayerHUD`
  (returns (GameplayHUD :type "/Game/FPS_AnimBP_v2/Widgets/W_HUD Object Reference"))
  (bind _gameplayhud (message `/Game/FPS_AnimBP_v2/Blueprints/Interfaces/BP_ControllerInterface.GetGameplayHUD` (`GameplayStatics.GetPlayerController` null)))
  (return _gameplayhud))

(fn `IsWeaponAttachmentAllowed`
  (params (AttachmentDataAsset :type "/Game/FPS_AnimBP_v2/Blueprints/DataAssets/Attachments/FPS_PDA_AttachmentDataBase Object Reference") (WeaponAttachments :type "/Game/FPS_AnimBP_v2/Data/Structs/Attachments/ST_WeaponAttachments Structure (by ref)") (`Gun Data Asset` :type "/Game/FPS_AnimBP_v2/Blueprints/DataAssets/Weapons/Guns/FPS_PDA_GunBase Object Reference"))
  (returns (ReturnValue :type Boolean))
  (bind ((`DisallowedAttachmentSlots_22_DBB976EF4F2D7510D2BB53BE56DD1B4D` _disallowedattachmentslots) (`DisallowedSpecificAttachments_25_347004694D0E8DC67EDCF4ABB0838977` _disallowedspecificattachments)) (break `/Game/FPS_AnimBP_v2/Data/Structs/Attachments/ST_WeaponAttachments` WeaponAttachments))
  (bind _allowedguns (`/Game/FPS_AnimBP_v2/Blueprints/DataAssets/Attachments/FPS_PDA_AttachmentDataBase.AllowedGuns` (`local.AttachmentDataAsset`)))
  ;[0 0 0] Check to see if the attachment is allowed to be equipped on this weapon
  (`/Engine/EditorBlueprintResources/StandardMacros.IsValid` AttachmentDataAsset
    (:`Is Valid`
      (return (and (and (not (`BlueprintSetLibrary.Set_Contains` _disallowedattachmentslots (`.AttachmentSlot` (`/Game/FPS_AnimBP_v2/Blueprints/DataAssets/Attachments/FPS_PDA_AttachmentDataBase.GetAttachmentBaseData` AttachmentDataAsset)))) (not (`BlueprintSetLibrary.Set_Contains` _disallowedspecificattachments (`local.AttachmentDataAsset`)))) (or (== (`KismetArrayLibrary.Array_Length` _allowedguns) 0) (`KismetArrayLibrary.Array_Contains` _allowedguns (`local.Gun Data Asset`))))))
    (:`Is Not Valid`
      (return false))))

(fn `LoadAssetBlockingPure`
  (params (Asset :type "Object Soft Object Reference"))
  (returns (ReturnValue :type "Object Object Reference"))
  (bind _returnvalue (`KismetSystemLibrary.LoadAsset_Blocking` Asset))
  (return _returnvalue))

(fn `LoadSoftAnimMontage`
  (params (`Soft Montage` :type "AnimMontage Soft Object Reference"))
  (returns (Montage :type "AnimMontage Object Reference"))
  (bind _returnvalue (`KismetSystemLibrary.LoadAsset_Blocking` `Soft Montage`))
  (bind _asanim_montage (cast `AnimMontage` _returnvalue))
  (return _asanim_montage))

(fn `LoadSoftAnimSequence`
  (params (`Soft Sequence` :type "AnimSequence Soft Object Reference"))
  (returns (Sequence :type "AnimSequence Object Reference"))
  (bind _returnvalue (`KismetSystemLibrary.LoadAsset_Blocking` `Soft Sequence`))
  (bind _asanim_sequence (cast `AnimSequence` _returnvalue))
  (return _asanim_sequence))

(fn `LoadSoftBlendSpace1D`
  (params (`Soft BS1D` :type "BlendSpace1D Soft Object Reference"))
  (returns (BS1D :type "BlendSpace1D Object Reference"))
  (bind _returnvalue (`KismetSystemLibrary.LoadAsset_Blocking` `Soft BS1D`))
  (bind _asblend_space_1d (cast `BlendSpace1D` _returnvalue))
  (return _asblend_space_1d))

(fn `LoadSoftSkeletalMesh`
  (params (`Soft Skeletal Mesh` :type "SkeletalMesh Soft Object Reference"))
  (returns (`Skeletal Mesh` :type "SkeletalMesh Object Reference"))
  (bind _returnvalue (`KismetSystemLibrary.LoadAsset_Blocking` `Soft Skeletal Mesh`))
  (bind _asskeletal_mesh (cast `SkeletalMesh` _returnvalue))
  (return _asskeletal_mesh))

(fn `LoadSoftSoundBase`
  (params (`Soft Sound Base` :type "SoundBase Soft Object Reference"))
  (returns (`Sound Base` :type "SoundBase Object Reference"))
  (bind _returnvalue (`KismetSystemLibrary.LoadAsset_Blocking` `Soft Sound Base`))
  (bind _assound_base (cast `SoundBase` _returnvalue))
  (return _assound_base))

(fn `LoadSoftSoundCue`
  (params (`Soft Sound Cue` :type "SoundBase Soft Object Reference"))
  (returns (`Sound Cue` :type "SoundCue Object Reference"))
  (bind _returnvalue (`KismetSystemLibrary.LoadAsset_Blocking` `Soft Sound Cue`))
  (bind _assound_cue (cast `SoundCue` _returnvalue))
  (return _assound_cue))

(fn `UpdateInputDevice`
  (params (Key :type "Key Structure" :default "None"))
  (message `/Game/FPS_AnimBP_v2/Blueprints/Interfaces/BP_ControllerInterface.OnAnyKeyPress` (`GameplayStatics.GetPlayerController` null) Key))
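; Player camera manager for the FPS character that relays player state to its camera modifiers, which control settings like FOV.
; On initialization it caches the FPS camera modifier, then forwards movement speed, aiming state, weapon ADS timings and default and target FOV to it.
; Entering the inventory preview adds a menu modifier and disables the FPS one so the preview FOV applies; exiting removes it and re-enables gameplay FOV.
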(event `InitializeCameraManager`
  ;[0 0 0] Begin Play - Set a reference to the Camera Modifier used to control camera settings like FOV
  (bind _returnvalue (`self.FindCameraModifierByClass` "/Game/FPS_AnimBP_v2/Blueprints/Camera/BP_CameraModifier_FPS.BP_CameraModifier_FPS_C"))
  (bind _asbp_camera_modifier_fps (cast `/Game/FPS_AnimBP_v2/Blueprints/Camera/BP_CameraModifier_FPS` _returnvalue))
  (set `self.CameraModifier` _asbp_camera_modifier_fps))

(event `/Game/FPS_AnimBP_v2/Blueprints/Interfaces/BP_CameraAnimInterface.UpdateMovementSpeed`
  (params (MovementSpeed :type "/Game/FPS_AnimBP_v2/Data/Enums/E_MovementSpeed Enum" :default "NewEnumerator0"))
  ;[0 0 0] Update various values about the player character states and camera value within the camera modifier
  (bind _cameramodifier (`self.CameraModifier`)
    (:`then`
      (set `/Game/FPS_AnimBP_v2/Blueprints/Camera/BP_CameraModifier_FPS.MovementSpeed` MovementSpeed _cameramodifier))
    (:`else`)))

(event `/Game/FPS_AnimBP_v2/Blueprints/Interfaces/BP_CameraAnimInterface.OnEquipWeapon`
  (params (TimeToEnterADS :type "Float (single-precision)") (TimeToExitADS :type "Float (single-precision)"))
  ;[0 0 0] Update various values about the player character states and camera value within the camera modifier
  (bind _cameramodifier (`self.CameraModifier`)
    (:`then`
      (set `/Game/FPS_AnimBP_v2/Blueprints/Camera/BP_CameraModifier_FPS.TimeToEnterADS` TimeToEnterADS _cameramodifier)
      (set `/Game/FPS_AnimBP_v2/Blueprints/Camera/BP_CameraModifier_FPS.TimeToExitADS` TimeToExitADS _cameramodifier))
    (:`else`)))

(event `/Game/FPS_AnimBP_v2/Blueprints/Interfaces/BP_CameraAnimInterface.UpdateIsAiming`
  (params (IsAiming :type Boolean))
  ;[0 0 0] Update various values about the player character states and camera value within the camera modifier
  (bind _cameramodifier (`self.CameraModifier`)
    (:`then`
      (set `/Game/FPS_AnimBP_v2/Blueprints/Camera/BP_CameraModifier_FPS.IsAiming` IsAiming _cameramodifier))
    (:`else`)))

(event `/Game/FPS_AnimBP_v2/Blueprints/Interfaces/BP_CameraAnimInterface.UpdateDefaultFOV`
  (params (`New Default FOV` :type "Float (single-precision)"))
  ;[0 0 0] Update various values about the player character states and camera value within the camera modifier
  (bind _cameramodifier (`self.CameraModifier`)
    (:`then`
      (set `/Game/FPS_AnimBP_v2/Blueprints/Camera/BP_CameraModifier_FPS.DefaultFOV` `New Default FOV` _cameramodifier))
    (:`else`)))

(event `/Game/FPS_AnimBP_v2/Blueprints/Interfaces/BP_CameraAnimInterface.UpdateTargetFOV`
  (params (`New Target FOV` :type "Float (single-precision)"))
  ;[0 0 0] Update various values about the player character states and camera value within the camera modifier
  (bind _cameramodifier (`self.CameraModifier`)
    (:`then`
      (set `/Game/FPS_AnimBP_v2/Blueprints/Camera/BP_CameraModifier_FPS.TargetFOV` `New Target FOV` _cameramodifier))
    (:`else`)))

(event `/Game/FPS_AnimBP_v2/Blueprints/Interfaces/BP_CameraAnimInterface.OnEnterExitPreviewMenu`
  (params (EnterMenu :type Boolean))
  ;[0 0 0] When the Inventory Menu is opened, override the Camera Modifier to allow the Preview FOV to be used rather than the gameplay FOV
  (if EnterMenu
    (bind _returnvalue (`self.AddNewCameraModifier` "/Game/FPS_AnimBP_v2/Blueprints/Camera/BP_CameraModifier_Menu.BP_CameraModifier_Menu_C"))
    (set `self.MenuCameraModifier` _returnvalue)
    (`CameraModifier.DisableModifier` (`self.CameraModifier`) true)
    (else
      (bind _menucameramodifier (`self.MenuCameraModifier`)
        (:`then`
          (`self.RemoveCameraModifier` _menucameramodifier)
          (`CameraModifier.EnableModifier` (`self.CameraModifier`)))
        (:`else`)))))

(fn `GetDefaultFOV`
  (returns (`Default FOV` :type "Float (double-precision)"))
  (return (`/Game/FPS_AnimBP_v2/Blueprints/Camera/BP_CameraModifier_FPS.DefaultFOV` (`self.CameraModifier`))))

(fn `UserConstructionScript`)
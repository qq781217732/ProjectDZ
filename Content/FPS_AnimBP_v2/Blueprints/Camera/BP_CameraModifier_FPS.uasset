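; Camera modifier for a first-person character that adjusts FOV and vignette for aiming down sights and sprinting.
; ADS and sprint alphas advance at constant rates from transition times, then nested ease-in-out blends move FOV toward the aim target and widen it proportionally while sprinting.
; The post-process pass separately interpolates vignette strength in while aiming and out otherwise.
; View location and rotation pass through unchanged.
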(fn `BlueprintModifyCamera`
  (params (DeltaTime :type "Float (single-precision)") (ViewLocation :type "Vector Structure") (ViewRotation :type "Rotator Structure") (FOV :type "Float (single-precision)"))
  (returns (NewViewLocation :type "Vector Structure") (NewViewRotation :type "Rotator Structure") (NewFOV :type "Float (single-precision)"))
  (bind _result (`|EaseFunction` "EaseInOut" (`self.ADS_Alpha`) (`self.DefaultFOV`) (`self.TargetFOV`) 2.5))
  (`|ExecutionSequence`
    (:`then_0`
      ;[0 0 0] Calculate the smooth FOV transition for ADS and sprinting
      (set `self.ADS_Alpha` (`KismetMathLibrary.FInterpTo_Constant` (`self.ADS_Alpha`) (select `bool` (`self.IsAiming`) :`true` 1.0) (`local.DeltaTime`) (/ 1.0 (select `bool` (`self.IsAiming`) :`false` (`self.TimeToExitADS`) :`true` (`self.TimeToEnterADS`)))))
      (set `self.SprintAlpha` (`KismetMathLibrary.FInterpTo_Constant` (`self.SprintAlpha`) (select `/Game/FPS_AnimBP_v2/Data/Enums/E_MovementSpeed` (`self.MovementSpeed`) :`NewEnumerator2` 1.0) (`local.DeltaTime`) (/ 1.0 (select `/Game/FPS_AnimBP_v2/Data/Enums/E_MovementSpeed` (`self.MovementSpeed`) :`NewEnumerator0` 0.2 :`NewEnumerator1` 0.2 :`NewEnumerator2` (`self.SprintFOV_InterpSpeedSeconds`))))))
    (:`then_1`
      ;[0 0 0] Ease the camera FOV in and out of the target values
      (return (`local.ViewLocation`) (`local.ViewRotation`) (`|EaseFunction` "EaseInOut" (`self.SprintAlpha`) _result (* _result 1.1))))))

(fn `BlueprintModifyPostProcess`
  (params (DeltaTime :type "Float (single-precision)"))
  (returns (PostProcessBlendWeight :type "Float (single-precision)") (PostProcessSettings :type "PostProcessSettings Structure"))
  (locals (local_InterpSpeed :type "Float (double-precision)" :default 0.0))
  ;[0 0 0] Controls the strength of the vignette effect while aiming down sights
  (bind _output_get (set `self.CurrentVignetteStrength` (`KismetMathLibrary.FInterpTo` (`self.CurrentVignetteStrength`) (select `bool` (`self.IsAiming`) :`true` 0.5) (`local.DeltaTime`) (/ 1.0 (select `bool` (`self.IsAiming`) :`false` (`self.TimeToExitADS`) :`true` (`self.TimeToEnterADS`))))))
  (return 1.0 (make `PostProcessSettings` :`VignetteIntensity` _output_get)))